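; Paper2D spike trap that endlessly retracts and extends, damaging actors that begin overlapping its box.
; BeginPlay runs a looping cycle, using a fixed delay to cover each animation and a Duration variable to hold each state.
; Down and up events step through four sprites with short delays.
; Box collision switches off once fully down and back on once fully up.
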(event OnComponentBeginOverlap(Box)
  (params (OverlappedComponent :type Primitive%20Component%20Object%20Reference) (OtherActor :type Actor%20Object%20Reference) (OtherComp :type Primitive%20Component%20Object%20Reference) (OtherBodyIndex :type Integer) (bFromSweep :type Boolean) (SweepResult :type Hit%20Result%20Structure%20%28by%20ref%29))
  (Game|Damage|ApplyDamage OtherActor 1.0 0 0))

(event Custom|BringSpikeDown
  (Rendering|Components|Sprite|SetSprite (Variables|Default|GetPaperSprite) "/Game/Assets/Tiles/sprite_0_Sprite.sprite_0_Sprite")
  (Utilities|FlowControl|Delay 0.1)
  (Rendering|Components|Sprite|SetSprite (Variables|Default|GetPaperSprite) "/Game/Assets/Tiles/sprite_1_Sprite.sprite_1_Sprite")
  (Utilities|FlowControl|Delay 0.1)
  (Rendering|Components|Sprite|SetSprite (Variables|Default|GetPaperSprite) "/Game/Assets/Tiles/sprite_2_Sprite.sprite_2_Sprite")
  (Utilities|FlowControl|Delay 0.1)
  (Rendering|Components|Sprite|SetSprite (Variables|Default|GetPaperSprite) "/Game/Assets/Tiles/sprite_3_Sprite.sprite_3_Sprite")
  (Collision|SetCollisionEnabled (Variables|Default|GetBox) "NoCollision"))

(event Custom|BringSpikeUp
  (Rendering|Components|Sprite|SetSprite (Variables|Default|GetPaperSprite) "/Game/Assets/Tiles/sprite_3_Sprite.sprite_3_Sprite")
  (Utilities|FlowControl|Delay 0.1)
  (Rendering|Components|Sprite|SetSprite (Variables|Default|GetPaperSprite) "/Game/Assets/Tiles/sprite_2_Sprite.sprite_2_Sprite")
  (Utilities|FlowControl|Delay 0.1)
  (Rendering|Components|Sprite|SetSprite (Variables|Default|GetPaperSprite) "/Game/Assets/Tiles/sprite_1_Sprite.sprite_1_Sprite")
  (Utilities|FlowControl|Delay 0.1)
  (Rendering|Components|Sprite|SetSprite (Variables|Default|GetPaperSprite) "/Game/Assets/Tiles/sprite_0_Sprite.sprite_0_Sprite")
  (Collision|SetCollisionEnabled (Variables|Default|GetBox) "QueryAndPhysics"))

(event EventBeginPlay
  (|CallParentFunction)
  (CallFunction|BringSpikeDown :!label _label)
  (Utilities|FlowControl|Delay 0.4)
  (Utilities|FlowControl|Delay (Variables|Default|GetDuration))
  (CallFunction|BringSpikeUp)
  (Utilities|FlowControl|Delay 0.4)
  (Utilities|FlowControl|Delay (Variables|Default|GetDuration))
  (goto _label))

(event Collision|EventActorBeginOverlap
  (params (OtherActor :type Actor%20Object%20Reference))
  (|CallParentFunction OtherActor) ; This node is disabled and will not be called.\nDrag off pins to build functionality.
)

(event EventTick
  (params (DeltaSeconds :type Float%20%28single-precision%29))
  (|CallParentFunction DeltaSeconds) ; This node is disabled and will not be called.\nDrag off pins to build functionality.
)

(fn ConstructionScript
  (|CallParentFunction))